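; Key pickup actor that unlocks its assigned Door_Blueprint when used from inside its trigger box.
; Box overlap toggles input; the Use action drives the logic, while the touch and E paths sit behind a false branch.
; With a single assigned door, it unlocks it, hides the key, briefly shows a pickup widget with the door name, then destroys itself.
; Multiple assigned doors only print a throttled message.
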(event OnComponentBeginOverlap(Box)
  (params (OverlappedComponent :type Primitive%20Component%20Object%20Reference) (OtherActor :type Actor%20Object%20Reference) (OtherComp :type Primitive%20Component%20Object%20Reference) (OtherBodyIndex :type Integer) (bFromSweep :type Boolean) (SweepResult :type Hit%20Result%20Structure%20%28by%20ref%29))
  ;[1 1 1] Player in Trigger?
  (Input|EnableInput (Game|GetPlayerController 0)))

(event OnComponentEndOverlap(Box)
  (params (OverlappedComponent :type Primitive%20Component%20Object%20Reference) (OtherActor :type Actor%20Object%20Reference) (OtherComp :type Primitive%20Component%20Object%20Reference) (OtherBodyIndex :type Integer))
  ;[1 1 1] Player in Trigger?
  (Input|DisableInput (Game|GetPlayerController 0)))

(event EventBeginPlay
  (bind _returnvalue (UserInterface|CreateWidget "/Game/SimpleDoorLockSystem/UMG´s/PickedUpText.PickedUpText_C"))
  ;[1 1 1] Change the ZOrder to what ever you want
  (UserInterface|Viewport|AddtoViewport _returnvalue 0))

(event Input|ActionEvents|InputActionUse
  (params (Key :type Key%20Structure :default "AnyKey"))
  (bind _door_blueprint (Variables|Default|GetDoor_Blueprint))
  ;[1 1 1] Unlocks the Door
  (:Pressed
    (for _array_element _door_blueprint
      (bind _asdoor_blueprint (Utilities|Casting|CastToDoor_Blueprint _array_element))
      (if (< (Utilities|Array|LastIndex _door_blueprint) 1)
        (Utilities|FlowControl|DoOnce false
          (:Completed
            (Default|Unlock _asdoor_blueprint)
            (Rendering|Components|TextRender|SetText (Variables|/Game/SimpleDoorLockSystem/UMG´s/PickedUpText.PickedUpText_C|GetKeyText (stale EventBeginPlay _returnvalue)) (Utilities|Text|ToText(Name) (Variables|/Game/SimpleDoorLockSystem/Blueprints/Door_Blueprint.Door_Blueprint_C|GetDoor_Name _asdoor_blueprint)))
            (Rendering|SetVisibility (Variables|Default|GetKey) false false)
            (Collision|SetCollisionEnabled (Variables|Default|GetKey) "NoCollision")
            (Widget|SetVisibility (Variables|/Game/SimpleDoorLockSystem/UMG´s/PickedUpText.PickedUpText_C|GetHorizontalBox_428 (stale EventBeginPlay _returnvalue)) "Visible")
            ;;[1 1 1] The time that the message is displayed
            (Utilities|FlowControl|Delay 1.5)
            (Widget|SetVisibility (Variables|/Game/SimpleDoorLockSystem/UMG´s/PickedUpText.PickedUpText_C|GetHorizontalBox_428 (stale EventBeginPlay _returnvalue)) "Hidden")
            (Actor|DestroyActor)))
        (else
          (Utilities|FlowControl|DoOnce false :!label _label
            (:Completed
              (Development|PrintString (Utilities|String|Append (Variables|Default|GetAppendText1) (Variables|Default|GetAppendText2)) true true "(R=1.000000,G=0.015237,B=0.000000,A=1.000000)" 99999.0)
              (Utilities|FlowControl|Delay 0.2)
              (goto _label Reset))))))))

(event Input|KeyboardEvents|E
  (params (Key :type Key%20Structure :default "AnyKey"))
  (bind _door_blueprint (Variables|Default|GetDoor_Blueprint))
  ;[1 1 1] Unlocks the Door
  (:Pressed
    (if false
      (for _array_element _door_blueprint
        (bind _asdoor_blueprint (Utilities|Casting|CastToDoor_Blueprint _array_element))
        (if (< (Utilities|Array|LastIndex _door_blueprint) 1)
          (Utilities|FlowControl|DoOnce false
            (:Completed
              (Default|Unlock _asdoor_blueprint)
              (Rendering|Components|TextRender|SetText (Variables|/Game/SimpleDoorLockSystem/UMG´s/PickedUpText.PickedUpText_C|GetKeyText (stale EventBeginPlay _returnvalue)) (Utilities|Text|ToText(Name) (Variables|/Game/SimpleDoorLockSystem/Blueprints/Door_Blueprint.Door_Blueprint_C|GetDoor_Name _asdoor_blueprint)))
              (Rendering|SetVisibility (Variables|Default|GetKey) false false)
              (Collision|SetCollisionEnabled (Variables|Default|GetKey) "NoCollision")
              (Widget|SetVisibility (Variables|/Game/SimpleDoorLockSystem/UMG´s/PickedUpText.PickedUpText_C|GetHorizontalBox_428 (stale EventBeginPlay _returnvalue)) "Visible")
              ;;[1 1 1] The time that the message is displayed
              (Utilities|FlowControl|Delay 1.5)
              (Widget|SetVisibility (Variables|/Game/SimpleDoorLockSystem/UMG´s/PickedUpText.PickedUpText_C|GetHorizontalBox_428 (stale EventBeginPlay _returnvalue)) "Hidden")
              (Actor|DestroyActor)))
          (else
            (Utilities|FlowControl|DoOnce false :!label _label
              (:Completed
                (Development|PrintString (Utilities|String|Append (Variables|Default|GetAppendText1) (Variables|Default|GetAppendText2)) true true "(R=1.000000,G=0.015237,B=0.000000,A=1.000000)" 99999.0)
                (Utilities|FlowControl|Delay 0.2)
                (goto _label Reset)))))))))

(event Input|TouchEvents|InputTouch
  (params (Location :type Vector) (FingerIndex :type ETouchIndex%20Enum))
  (bind _door_blueprint (Variables|Default|GetDoor_Blueprint))
  (bind _key (Variables|Default|GetKey))
  ;[1 1 1] Unlocks the Door
  (:Pressed
    (if false
      (for _array_element _door_blueprint
        (bind _asdoor_blueprint (Utilities|Casting|CastToDoor_Blueprint _array_element))
        (if (< (Utilities|Array|LastIndex _door_blueprint) 1)
          (Utilities|FlowControl|DoOnce false
            (:Completed
              (Default|Unlock _asdoor_blueprint)
              (Rendering|Components|TextRender|SetText (Variables|/Game/SimpleDoorLockSystem/UMG´s/PickedUpText.PickedUpText_C|GetKeyText (stale EventBeginPlay _returnvalue)) (Utilities|Text|ToText(Name) (Variables|/Game/SimpleDoorLockSystem/Blueprints/Door_Blueprint.Door_Blueprint_C|GetDoor_Name _asdoor_blueprint)))
              (Rendering|SetVisibility _key false false)
              (Collision|SetCollisionEnabled _key "NoCollision")
              (Widget|SetVisibility (Variables|/Game/SimpleDoorLockSystem/UMG´s/PickedUpText.PickedUpText_C|GetHorizontalBox_428 (stale EventBeginPlay _returnvalue)) "Visible")
              ;;[1 1 1] The time that the message is displayed
              (Utilities|FlowControl|Delay 1.5)
              (Widget|SetVisibility (Variables|/Game/SimpleDoorLockSystem/UMG´s/PickedUpText.PickedUpText_C|GetHorizontalBox_428 (stale EventBeginPlay _returnvalue)) "Hidden")
              (Actor|DestroyActor)))
          (else
            (Utilities|FlowControl|DoOnce false :!label _label
              (:Completed
                (Development|PrintString (Utilities|String|Append (Variables|Default|GetAppendText1) (Variables|Default|GetAppendText2)) true true "(R=1.000000,G=0.015237,B=0.000000,A=1.000000)" 99999.0)
                (Utilities|FlowControl|Delay 0.2)
                (goto _label Reset)))))))))

(fn ConstructionScript)